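; Racing game mode that runs a timed checkpoint race, with a win at the finish line and a loss when time runs out.
; BeginPlay binds to every BP_Checkpoint, then a start countdown delay leads into the race timer.
; Regular checkpoints re-arm that timer with remaining plus bonus time and play the HUD's time-added animation.
; The finish line clears the timer; both outcomes call GameFinish, which is empty here.
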(event `self.ReceiveBeginPlay`
  (`|ExecutionSequence`
    (:`then_0`
      (bind _outactors (`GameplayStatics.GetAllActorsOfClass` "/Game/ShubhamShrey/Checkpoints/BP_Checkpoint.BP_Checkpoint_C"))
      (for _array_element _outactors
        (if (`/Game/ShubhamShrey/Checkpoints/BP_Checkpoint. IsFinishLine` _array_element)
          (add `/Game/ShubhamShrey/Checkpoints/BP_Checkpoint.OnCheckpointCrossed` _array_element (delegate `Win_CrossTheFinishLine`))
          (else
            (add `/Game/ShubhamShrey/Checkpoints/BP_Checkpoint.OnCheckpointCrossedWithTime` _array_element (delegate `CrossedACheckpoint`))))))
    (:`then_1`
      (`self.Start Countdown`))))

(event `Start Countdown`
  (`KismetSystemLibrary.Delay` (`self.StartCountdownDuration`))
  (`self.Game Start`))

(event `Game Start`
  (bind _returnvalue (`KismetSystemLibrary.K2_SetTimerDelegate` (delegate `LoseOutOfTime`) (`self.StartTimerDuration`)))
  (set `self.TimeRemainingTimer` _returnvalue))

(event `LoseOutOfTime`
  (`self.Game Finish` false))

(event `Win_CrossTheFinishLine`
  (`KismetSystemLibrary.K2_ClearAndInvalidateTimerHandle` (`self.TimeRemainingTimer`))
  (`self.Game Finish` true))

(event `Game Finish`
  (params (Win :type Boolean)))

(event `CrossedACheckpoint`
  (params (TimeToAdd :type Integer))
  (`self.AddTimeToTimer` TimeToAdd))

(fn `AddTimeToTimer`
  (params (TimeToAdd :type Integer))
  (bind _returnvalue (`KismetSystemLibrary.K2_SetTimerDelegate` (`|CreateDelegate` :!event `LoseOutOfTime`) (+ (`KismetSystemLibrary.K2_GetTimerRemainingTimeHandle` (`self.TimeRemainingTimer`)) (`local.TimeToAdd`))))
  (set `self.TimeRemainingTimer` _returnvalue)
  (bind _asvehicle_player_controller (cast `/Game/VehicleTemplate/Blueprints/VehiclePlayerController` (`GameplayStatics.GetPlayerController` 0)))
  (`/Game/VehicleTemplate/Blueprints/VehicleUI.PlayTimeAddedAnim` (`/Game/VehicleTemplate/Blueprints/VehiclePlayerController.VehicleHud` _asvehicle_player_controller)))

(fn `UserConstructionScript`)