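; BP_Speedometer is an in-world dashboard gauge for the SportsCar pawn, showing engine RPM, speed in MPH and current gear.
; On BeginPlay it caches its parent actor as the owning vehicle, then polls that vehicle's movement component every Tick.
; RPM drives a text-render needle's roll and high-rev red tint.
; Speed and gear texts change color with direction or gear state, with R and N labels for reverse and neutral.
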(event `self.ReceiveBeginPlay`
  (bind _assports_car_pawn (cast `/Game/VehicleTemplate/Blueprints/SportsCar/SportsCar_Pawn` (`self.GetParentActor`)))
  (set `self.Owning Vehicle` _assports_car_pawn))

(event `self.ReceiveTick`
  (params (DeltaSeconds :type "Float (single-precision)"))
  (bind _speed_text (`self.Speed_Text`))
  (bind _rpm_needle (`self.RPM_Needle`))
  (bind _gear_text (`self.Gear_Text`))
  (bind _movement_component_variable (`/Game/VehicleTemplate/Blueprints/SportsCar/SportsCar_Pawn.Movement Component Variable` (`self.Owning Vehicle`)))
  (bind _returnvalue (`ChaosVehicleMovementComponent.GetCurrentGear` _movement_component_variable))
  (bind _returnvalue_2 (`ChaosWheeledVehicleMovementComponent.GetEngineRotationSpeed` _movement_component_variable))
  (bind _returnvalue_3 (`ChaosVehicleMovementComponent.GetForwardSpeedMPH` _movement_component_variable))
  (bind _returnvalue_4 (+ _returnvalue 1))
  (bind _returnvalue_5 (< _returnvalue 1))
  (`SceneComponent.K2_SetRelativeRotation` _rpm_needle (`KismetMathLibrary.MakeRotator` (`KismetMathLibrary.MapRangeClamped` _returnvalue_2 0.0 (`ChaosWheeledVehicleMovementComponent.GetEngineMaxRotationSpeed` _movement_component_variable) 48.043821 -212.258407)) false false)
  (`TextRenderComponent.SetTextRenderColor` _rpm_needle (select `bool` (> _returnvalue_2 5000.0) :`false` (make `Color` 255 255 255 50) :`true` (`KismetMathLibrary.Conv_LinearColorToColor` (`KismetMathLibrary.MakeColor` (`KismetMathLibrary.MapRangeClamped` _returnvalue_2 5000.0 7000.0 0.0 1.0) 0.0 0.0 0.2))))
  (`TextRenderComponent.K2_SetText` _speed_text (`KismetTextLibrary.Conv_IntToText` (`KismetMathLibrary.Round` (`KismetMathLibrary.Abs` _returnvalue_3))))
  (`TextRenderComponent.SetTextRenderColor` _speed_text (select `int` (+ (`KismetMathLibrary.Round` (`KismetMathLibrary.SignOfFloat` _returnvalue_3)) 1) :`0` (make `Color` 0 0 255 50) :`1` (make `Color` 255 255 255 50) :`2` (make `Color` 0 200 0 50)))
  (`TextRenderComponent.K2_SetText` _gear_text (select `bool` _returnvalue_5 :`false` (`KismetTextLibrary.Conv_IntToText` _returnvalue) :`true` (select `int` _returnvalue_4 :`0` "R" :`1` "N")))
  (`TextRenderComponent.SetTextRenderColor` _gear_text (select `bool` _returnvalue_5 :`false` (make `Color` 0 255 0 50) :`true` (select `int` _returnvalue_4 :`0` (make `Color` 0 0 255 50) :`1` (make `Color` 255 255 255 50)))))

(fn `UserConstructionScript`)